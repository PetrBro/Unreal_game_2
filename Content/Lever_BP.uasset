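; Lever actor that lets the player open a door when within range.
; On BeginPlay it adds an F-button prompt widget to the viewport and caches the Door_BP found by GetActorOfClass.
; Box overlaps show and hide the prompt, whose visibility doubles as the range check.
; The OpenDoor event, triggered from outside this graph, snaps the door to a fixed raised position without animation or any closing logic.
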(event `self.ReceiveBeginPlay`
  (bind _returnvalue (`|CreateWidget` "/Game/F_button_widget.F_button_widget_C"))
  (bind _output_get (set `self.Button Wig Ref` _returnvalue))
  (`UserWidget.AddToViewport` _output_get 0)
  (bind _returnvalue_2 (`GameplayStatics.GetActorOfClass` "/Game/Door_BP.Door_BP_C"))
  (set `self.Door Bp Ref` _returnvalue_2))

(event `self.Box.OnComponentBeginOverlap`
  (params (OverlappedComponent :type "PrimitiveComponent Object Reference") (OtherActor :type "Actor Object Reference") (OtherComp :type "PrimitiveComponent Object Reference") (OtherBodyIndex :type Integer) (bFromSweep :type Boolean) (SweepResult :type "HitResult Structure (by ref)"))
  (`Widget.SetVisibility` (`self.Button Wig Ref`) "Visible"))

(event `self.Box.OnComponentEndOverlap`
  (params (OverlappedComponent :type "PrimitiveComponent Object Reference") (OtherActor :type "Actor Object Reference") (OtherComp :type "PrimitiveComponent Object Reference") (OtherBodyIndex :type Integer))
  (`Widget.SetVisibility` (`self.Button Wig Ref`) "Hidden"))

(event `Open Door`
  (if (`Widget.IsVisible` (`self.Button Wig Ref`))
    (`SceneComponent.K2_SetRelativeLocation` (`/Game/Door_BP.Door` (`self.Door Bp Ref`)) (0.0 0.0 420.0) false false)))

(fn `UserConstructionScript`)